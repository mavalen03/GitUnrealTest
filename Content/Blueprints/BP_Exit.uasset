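; BP_Exit is a level exit that opens the win screen when the player arrives with the required egg count.
; BeginPlay sets that count from a hardcoded level-name chain and prints it.
; On overlap by BP_ControllableCharacter, an exact match either shows an existing WinScreen and pauses, or only creates WBP_Win if none exists yet.
; A mismatch prints a not-enough-eggs message.
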(event `self.ReceiveBeginPlay`
  (bind _returnvalue (`GameplayStatics.GetCurrentLevelName` true))
  (set `self.LevelName` _returnvalue)
  (if (`KismetStringLibrary.EqualEqual_StrStr` (`self.LevelName`) "TestLevel")
    (set `self.NeededEggs` 3)
    (`KismetSystemLibrary.PrintString` "3 Eggs Needed")
    (elif (`KismetStringLibrary.EqualEqual_StrStr` (`self.LevelName`) "Level1")
      (set `self.NeededEggs` 1)
      (`KismetSystemLibrary.PrintString` "1 Egg Needed")
      (elif (`KismetStringLibrary.EqualEqual_StrStr` (`self.LevelName`) "Level2")
        (set `self.NeededEggs` 1)
        (`KismetSystemLibrary.PrintString` "1 Egg Needed")
        (elif (`KismetStringLibrary.EqualEqual_StrStr` (`self.LevelName`) "Level3")
          (set `self.NeededEggs` 1)
          (`KismetSystemLibrary.PrintString` "1 Egg Needed"))))))

(event `self.ReceiveActorBeginOverlap`
  (params (OtherActor :type "Actor Object Reference"))
  (bind _winscreen (`self.WinScreen`))
  (bind _returnvalue (`GameplayStatics.GetActorOfClass` "/Game/Blueprints/BP_ControllableCharacter.BP_ControllableCharacter_C"))
  (if (== _returnvalue OtherActor)
    (bind _returnvalue_2 (`ControllableCharacter.GetNumEggs` _returnvalue))
    (if (== _returnvalue_2 (`self.NeededEggs`))
      (`/Engine/EditorBlueprintResources/StandardMacros.IsValid` _winscreen
        (:`Is Valid`
          (`UserWidget.AddToViewport` _winscreen 0)
          (`GameplayStatics.SetGamePaused` true))
        (:`Is Not Valid`
          (bind _returnvalue_3 (`|CreateWidget` "/Game/UI/WBP_Win.WBP_Win_C"))
          (set `self.WinScreen` _returnvalue_3)))
      (else
        (`KismetSystemLibrary.PrintString` "Not Enough Eggs")))))

(fn `UserConstructionScript`)